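; BP_NavLink is a smart nav link that makes Enemy agents jump to the link's destination.
; When the link is reached, it casts the agent to Enemy and launches it, overriding its current velocity.
; CalculateVelocity solves the ballistic launch velocity that lands on the destination after Duration seconds, using a hard-coded gravity of 982 rather than the world setting.
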(event EventBeginPlay)

(event Collision|EventActorBeginOverlap
  (params (OtherActor :type Actor%20Object%20Reference)))

(event EventTick
  (params (DeltaSeconds :type Float%20%28single-precision%29)))

(event EventSmartLinkReached
  (params (Agent :type Actor%20Object%20Reference) (Destination :type Vector%20%28by%20ref%29 :default "0, 0, 0"))
  (bind _asenemy (Utilities|Casting|CastToEnemy Agent))
  (bind _velocity (CallFunction|CalculateVelocity Destination (Transformation|GetActorLocation _asenemy) (Variables|Default|GetDuration)))
  (Character|LaunchCharacter _asenemy _velocity true true))

(fn ConstructionScript)

(fn CalculateVelocity
  (params (Destination%20Location :type Vector) (Start%20Location :type Vector) (Duration :type Float%20%28double-precision%29))
  (bind (_x _y _z) (Math|Vector|BreakVector Start%20Location))
  (bind (_x_2 _y_2 _z_2) (Math|Vector|BreakVector Destination%20Location))
  ;[1 1 1] https://www.youtube.com/watch?v=wW4t5QxOQaE 무슨 공식인지 이해 못해서 그냥 따라함 zz.
  (LocalVariables|SetLocalDuration Duration)
  (return (Math|Vector|MakeVector (/ (- _x_2 _x) (LocalVariables|GetLocalDuration)) (/ (- _y_2 _y) (LocalVariables|GetLocalDuration)) (/ (- _z_2 (+ _z (* (Math|Float|Square (LocalVariables|GetLocalDuration)) -0.5 982.0))) (LocalVariables|GetLocalDuration)))))