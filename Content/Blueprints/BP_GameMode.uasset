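; Game mode that tracks the current and best score and runs the game-over sequence when the character dies.
; BeginPlay loads the best score from a save slot, and AddScore increments the score, saving whenever it beats the best.
; Death triggers slow motion, then a timer shows the end-game widget with UI-only input and cursor, and a second timer pauses the game.
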(event Custom|GamePause
  (Game|SetGamePaused true))

(event Custom|EndGame
  (bind _returnvalue (Game|GetPlayerController 0))
  (bind _returnvalue_2 (UserInterface|CreateWidget "/Game/UI/WBP_EndGameWidget.WBP_EndGameWidget_C"))
  (UserInterface|Viewport|AddtoViewport _returnvalue_2 0)
  (Input|SetInputModeUIOnly _returnvalue _returnvalue_2 "LockOnCapture" false)
  (Variables|/Script/Engine.PlayerController|SetbShowMouseCursor _returnvalue true)
  (Utilities|Time|SetTimerbyEvent (delegate Custom|GamePause) 1.0))

(event EventBeginPlay
  (bind _bestscore (CallFunction|LoadScoreData))
  (Variables|Default|SetBestScore _bestscore))

(event EventOnCharacterDie
  (Utilities|Time|SetGlobalTimeDilation 0.3)
  (Utilities|Time|SetTimerbyEvent (delegate Custom|EndGame) 0.5))

(fn ConstructionScript)

(fn AddScore
  (bind _result (Math|Integer|IncrementInt (Variables|Default|GetNowScore))
    (:%20%20
      (bind _output_get (Variables|Default|SetNowScore _result))
      (if (> _output_get (Variables|Default|GetBestScore))
        (bind _output_get_2 (Variables|Default|SetBestScore _output_get))
        (CallFunction|SaveScoreData _output_get_2)))))

(fn SaveScoreData
  (params (SaveValue :type Integer))
  (bind _returnvalue (SaveGame|CreateSaveGameObject "/Game/Blueprints/BP_SaveGame.BP_SaveGame_C"))
  (bind _output_get (Variables|Default|SetSaveInstance _returnvalue))
  (Variables|/Game/Blueprints/BP_SaveGame.BP_SaveGame_C|SetScoreData _output_get SaveValue)
  (SaveGame|SaveGametoSlot _output_get "BestScoreData"))

(fn LoadScoreData
  (bind _returnvalue (SaveGame|DoesSaveGameExist "BestScoreData"))
  (if _returnvalue
    (bind _returnvalue_2 (SaveGame|LoadGamefromSlot "BestScoreData"))
    (bind _asbp_save_game (Utilities|Casting|CastToBP_SaveGame _returnvalue_2))
    (return (Variables|/Game/Blueprints/BP_SaveGame.BP_SaveGame_C|GetScoreData _asbp_save_game))))